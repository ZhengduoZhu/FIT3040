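; Weapon equipment item for the inventory system that equips itself on the player when used.
; UseItem casts player 0 to ParentCharacter, has its InventoryComponent02 unequip one fixed equipment-type slot, then equips this item into that same slot.
; It returns whether the cast succeeded, and the event graph and construction script add no logic of their own.
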(fn `UseItem`
  (returns (Success :type Boolean))
  (bind _asparent_character (cast `/Game/ZhengduoZhu/Character/Player/ParentCharacter` (`GameplayStatics.GetPlayerCharacter` 0))
    (:`then`
      (bind _inventorycomponent02 (`/Game/ZhengduoZhu/Character/Player/ParentCharacter.InventoryComponent02` _asparent_character))
      (`/Game/ZhengduoZhu/InventorySystem02/InventoryComponent02.Unequip` _inventorycomponent02 "NewEnumerator3")
      (`/Game/ZhengduoZhu/InventorySystem02/InventoryComponent02.Equip` _inventorycomponent02 self "NewEnumerator3")
      (return true))
    (:`CastFailed`
      (return false))))

(fn `UserConstructionScript`
  (`parent.UserConstructionScript`))