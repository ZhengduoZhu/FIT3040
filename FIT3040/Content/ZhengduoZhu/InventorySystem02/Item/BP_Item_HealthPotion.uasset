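; Health potion item Blueprint in an inventory system that heals the player when used.
; It overrides UseItem to cast player 0 to ParentCharacter and add HealingPower to Health, clamped between zero and MaxHealth.
; On success it returns the parent UseItem result; a failed cast prints an error and returns false.
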(fn `UseItem`
  (returns (Success :type Boolean))
  (bind _asparent_character (cast `/Game/ZhengduoZhu/Character/Player/ParentCharacter` (`GameplayStatics.GetPlayerCharacter` 0))
    (:`then`
      (set `/Game/ZhengduoZhu/Character/Player/ParentCharacter.Health` (`KismetMathLibrary.FClamp` (+ (`/Game/ZhengduoZhu/Character/Player/ParentCharacter.Health` _asparent_character) (`self.HealingPower`)) 0.0 (`/Game/ZhengduoZhu/Character/Player/ParentCharacter.MaxHealth` _asparent_character)) _asparent_character)
      (bind _success (`parent.UseItem`))
      (return _success))
    (:`CastFailed`
      (`KismetSystemLibrary.PrintString` "Potion CAst character failed")
      (return false))))

(fn `UserConstructionScript`
  (`parent.UserConstructionScript`))