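; BP_Item is an item actor in an inventory system that is picked up through interaction.
; Interact adds the item's class and amount to the interactor's InventoryComponent02, which also creates obtain notifications for the quantity taken.
; Partial pickups leave the remainder on the actor, while full pickups destroy it.
; UseItem is a simple implementation that prints a message, destroys the actor and returns true.
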(event `/Game/ZhengduoZhu/InventorySystem/Interact_Interface.Interact`
  (params (Interactor :type "Actor Object Reference"))
  (bind _returnvalue (`self.GetComponentByClass` Interactor "/Game/ZhengduoZhu/InventorySystem02/InventoryComponent02.InventoryComponent02_C"))
  (bind (_iteminfo_name _iteminfo_description _iteminfo_icon _iteminfo_canbeused_ _iteminfo_usetext _iteminfo_canbestacked_ _iteminfo_maxstacksize _iteminfo_category _iteminfo_itemclass) (break `/Game/ZhengduoZhu/InventorySystem02/Blueprint/Structures/S_ItemInfo` (`self.ItemInfo`)))
  (bind (_iteminfo_name_2 _iteminfo_description_2 _iteminfo_icon_2 _iteminfo_canbeused__2 _iteminfo_usetext_2 _iteminfo_canbestacked__2 _iteminfo_maxstacksize_2 _iteminfo_category_2 _iteminfo_itemclass_2) (break `/Game/ZhengduoZhu/InventorySystem02/Blueprint/Structures/S_ItemInfo` (`self.ItemInfo`)))
  (`/Engine/EditorBlueprintResources/StandardMacros.IsValid` _returnvalue
    (:`Is Valid`
      (bind (_success _rest) (`/Game/ZhengduoZhu/InventorySystem02/InventoryComponent02.AddItem` _returnvalue _iteminfo_itemclass (`self.Amount`)))
      (if _success
        (if (> _rest 0)
          (`/Game/ZhengduoZhu/InventorySystem02/InventoryComponent02.CreateObtainNotifications` _returnvalue _iteminfo_itemclass_2 (- (`self.Amount`) _rest) (`self.ObtainDuration`))
          (set `self.Amount` _rest)
          (else
            (`/Game/ZhengduoZhu/InventorySystem02/InventoryComponent02.CreateObtainNotifications` _returnvalue _iteminfo_itemclass_2 (`self.Amount`) (`self.ObtainDuration`))
            (`self.K2_DestroyActor`)))))
    (:`Is Not Valid`
      (`KismetSystemLibrary.PrintString` "InventoryComponent02 Is not valied"))))

(fn `UseItem`
  (returns (Success :type Boolean))
  (`KismetSystemLibrary.PrintString` "Use Item")
  (`self.K2_DestroyActor`)
  (return true))

(fn `UserConstructionScript`)