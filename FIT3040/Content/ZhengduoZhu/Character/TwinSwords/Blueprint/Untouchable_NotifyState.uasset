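; Animation notify state that makes a character invulnerable for a span of an animation, in the TwinSwords character's folder.
; On begin it casts the mesh's owner to Character and sets CanBeDamaged to false; on end it sets it back to true.
; A failed cast only prints a debug message.
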(fn `Received_NotifyBegin`
  (params (MeshComp :type "SkeletalMeshComponent Object Reference") (Animation :type "AnimSequenceBase Object Reference") (TotalDuration :type "Float (double-precision)"))
  (returns (ReturnValue :type Boolean))
  (bind _ascharacter (cast `Character` (`ActorComponent.GetOwner` MeshComp))
    (:`then`
      (set `Actor.bCanBeDamaged` false _ascharacter)
      (return false))
    (:`CastFailed`
      (`KismetSystemLibrary.PrintString` null "UntouchableCastFailed!"))))

(fn `Received_NotifyEnd`
  (params (MeshComp :type "SkeletalMeshComponent Object Reference") (Animation :type "AnimSequenceBase Object Reference"))
  (returns (ReturnValue :type Boolean))
  (bind _ascharacter (cast `Character` (`ActorComponent.GetOwner` MeshComp))
    (:`then`
      (set `Actor.bCanBeDamaged` true _ascharacter)
      (return false))
    (:`CastFailed`
      (`KismetSystemLibrary.PrintString` null "UntouchableCastFailed!"))))