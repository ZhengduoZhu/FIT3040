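; Anim notify state that switches the TwinSwords player character to Flying movement for the duration of the notify window in an animation.
; Begin sets the CharacterMovement mode to Flying and End restores it to Walking.
; It targets player 0's character rather than the mesh owner, and prints an error if that character is not a TwinSwords.
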(fn `Received_NotifyBegin`
  (params (MeshComp :type "SkeletalMeshComponent Object Reference") (Animation :type "AnimSequenceBase Object Reference") (TotalDuration :type "Float (double-precision)"))
  (returns (ReturnValue :type Boolean))
  (bind _astwin_swords (cast `/Game/ZhengduoZhu/Character/TwinSwords/TwinSwords` (`GameplayStatics.GetPlayerCharacter` MeshComp))
    (:`then`
      (`CharacterMovementComponent.SetMovementMode` (`Character.CharacterMovement` _astwin_swords) "MOVE_Flying" 0)
      (return false))
    (:`CastFailed`
      (`KismetSystemLibrary.PrintString` null "NotifyStateError"))))

(fn `Received_NotifyEnd`
  (params (MeshComp :type "SkeletalMeshComponent Object Reference") (Animation :type "AnimSequenceBase Object Reference"))
  (returns (ReturnValue :type Boolean))
  (bind _astwin_swords (cast `/Game/ZhengduoZhu/Character/TwinSwords/TwinSwords` (`GameplayStatics.GetPlayerCharacter` MeshComp))
    (:`then`
      (`CharacterMovementComponent.SetMovementMode` (`Character.CharacterMovement` _astwin_swords) "MOVE_Walking" 0)
      (return false))
    (:`CastFailed`
      (`KismetSystemLibrary.PrintString` null "NotifyStateError"))))