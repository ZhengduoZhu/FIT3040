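; Anim notify state that opens a hit window for the TwinSwords character's right sword during an animation.
; On begin it sets RWeaponCollision to query-only collision, and on end it disables that collision.
; Both events cast player character 0 to TwinSwords rather than using the animated mesh's owner, and print a message if the cast fails.
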(fn `Received_NotifyBegin`
  (params (MeshComp :type "SkeletalMeshComponent Object Reference") (Animation :type "AnimSequenceBase Object Reference") (TotalDuration :type "Float (double-precision)"))
  (returns (ReturnValue :type Boolean))
  (bind _astwin_swords (cast `/Game/ZhengduoZhu/Character/TwinSwords/TwinSwords` (`GameplayStatics.GetPlayerCharacter` MeshComp))
    (:`then`
      (`PrimitiveComponent.SetCollisionEnabled` (`/Game/ZhengduoZhu/Character/TwinSwords/TwinSwords.R_WeaponCollision` _astwin_swords) "QueryOnly")
      (return false))
    (:`CastFailed`
      (`KismetSystemLibrary.PrintString` null "NotifyStateToggleCollisionCastFailed!"))))

(fn `Received_NotifyEnd`
  (params (MeshComp :type "SkeletalMeshComponent Object Reference") (Animation :type "AnimSequenceBase Object Reference"))
  (returns (ReturnValue :type Boolean))
  (bind _astwin_swords (cast `/Game/ZhengduoZhu/Character/TwinSwords/TwinSwords` (`GameplayStatics.GetPlayerCharacter` MeshComp))
    (:`then`
      (`PrimitiveComponent.SetCollisionEnabled` (`/Game/ZhengduoZhu/Character/TwinSwords/TwinSwords.R_WeaponCollision` _astwin_swords) "NoCollision")
      (return false))
    (:`CastFailed`
      (`KismetSystemLibrary.PrintString` null "NotifyStateToggleCollisionCastFailed!"))))